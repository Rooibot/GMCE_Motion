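; Motion matching player character Blueprint on GMC that adds aiming, strafing and traversal to its parent and creates an on-screen motion matching widget.
; Input queues abilities by tag, with jump becoming Traverse when a traversal solver is available.
; Tick adjusts pivot prediction for strafing and auto-queues traversal when toggled on.
; A test SV-to-MC event chain precalculates motion-warped montage paths, then plays the montage except on simulated proxies.
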(event Custom|SV_TestEvent
  (params (Montage :type Anim%20Montage%20Object%20Reference) (StartPosition :type Float%20%28double-precision%29) (PlayRate :type Float%20%28double-precision%29) (OriginTransform :type Transform) (MeshRelativeTransform :type Transform) (WarpTargets :type Array%20of%20GMCE%20Motion%20Warp%20Target%20Structures))
  (CallFunction|MCTestEvent Montage StartPosition PlayRate OriginTransform MeshRelativeTransform WarpTargets))

(event Custom|TestEvent
  (params (Montage :type Anim%20Montage%20Object%20Reference) (StartPosition :type Float%20%28double-precision%29) (PlayRate :type Float%20%28double-precision%29) (OriginTransform :type Transform) (MeshRelativeTransform :type Transform) (Targets :type Array%20of%20GMCE%20Motion%20Warp%20Target%20Structures))
  (CallFunction|SVTestEvent Montage StartPosition PlayRate OriginTransform MeshRelativeTransform Targets))

(event Custom|MC_TestEvent
  (params (Montage :type Anim%20Montage%20Object%20Reference) (StartPosition :type Float%20%28double-precision%29) (PlayRate :type Float%20%28double-precision%29) (OriginTransform :type Transform) (MeshRelativeTransform :type Transform) (WarpTargets :type Array%20of%20GMCE%20Motion%20Warp%20Target%20Structures))
  (bind _template_movement_component (Variables|Default|GetTemplate%20Movement%20Component))
  (if true
    (Class|GMCEMotionWarpingComponent|PrecalculatePathwithWarpTargets (Variables|Default|GetMotionWarpingComponent) Montage StartPosition PlayRate OriginTransform MeshRelativeTransform WarpTargets))
  (if (not (Class|GMCReplicationCmp|IsSimulatedProxy _template_movement_component))
    (Class|GMCMovementUtilityCmp|PlayMontageBlocking _template_movement_component (Variables|Default|GetMeshComponent) (Variables|/Script/GMCCore.GMC_OrganicMovementCmp|GetMontageTracker _template_movement_component) Montage StartPosition PlayRate true false true false "MontageLength")))

(event Input|EnhancedActionEvents|EnhancedInputActionIA_AutoTraverse
  (params (ActionValue :type Boolean) (ElapsedSeconds :type Float%20%28double-precision%29) (TriggeredSeconds :type Float%20%28double-precision%29) (InputAction :type Input%20Action%20Object%20Reference :default "/GMCE_Motion/Input/IA_AutoTraverse.IA_AutoTraverse"))
  (:Started
    (Variables|Default|SetWantsAutoTraverse (not (Variables|Default|GetWantsAutoTraverse)))))

(event Input|EnhancedActionEvents|EnhancedInputActionIA_ToggleStrafe
  (params (ActionValue :type Boolean) (ElapsedSeconds :type Float%20%28double-precision%29) (TriggeredSeconds :type Float%20%28double-precision%29) (InputAction :type Input%20Action%20Object%20Reference :default "/GMCE_Motion/Input/IA_ToggleStrafe.IA_ToggleStrafe"))
  (:Started
    (Class|GMCAbilitySystemComponent|QueueAbility (Variables|Default|GetAbilitySystemComponent) "(TagName=\"Ability.ToggleStrafe\")" InputAction)))

(event Input|EnhancedActionEvents|EnhancedInputActionIA_Aim
  (params (ActionValue :type Boolean) (ElapsedSeconds :type Float%20%28double-precision%29) (TriggeredSeconds :type Float%20%28double-precision%29) (InputAction :type Input%20Action%20Object%20Reference :default "/Game/GMASExtended/Input/IA_Aim.IA_Aim"))
  (:Started
    (Class|GMCAbilitySystemComponent|QueueAbility (Variables|Default|GetAbilitySystemComponent) "(TagName=\"Ability.Aim\")" InputAction)))

(event EventTick
  (params (DeltaSeconds :type Float%20%28single-precision%29))
  (bind _template_movement_component (Variables|Default|GetTemplate%20Movement%20Component))
  (|CallParentFunction DeltaSeconds)
  (Variables|/Script/GMCExtended.GMCE_OrganicMovementCmp|SetPivotPredictionAngleThreshold (Variables|Default|GetTemplate%20Movement%20Component) (Math|Float|SelectFloat 4e+01 6e+01 (Class|GMCAbilitySystemComponent|HasActiveTag (Variables|Default|GetAbilitySystemComponent) "(TagName=\"State.IsStrafing\")")))
  (if (Math|Boolean|ANDBoolean (Variables|Default|GetWantsAutoTraverse) (Class|GMCEOrganicMovementCmp|IsSolutionAvailableforSolver _template_movement_component "(TagName=\"Solver.Traversal\")") (AI|Components|NavMovement|IsMovingonGround _template_movement_component) (Class|GMCEOrganicMovementCmp|IsInputPresent (Variables|Default|GetTemplate%20Movement%20Component) false) (not (Class|GMCAbilitySystemComponent|HasActiveTag (Variables|Default|GetAbilitySystemComponent) "(TagName=\"Solver.Traversal\")")))
    (Class|GMCAbilitySystemComponent|QueueAbility (Variables|Default|GetAbilitySystemComponent) "(TagName=\"Ability.Traverse\")" 0)))

(fn ConstructionScript
  (|CallParentFunction)
  (bind _returnvalue (Game|ConstructObjectfromClass "/Script/GMCExtendedAnimation.GMCE_RootMotionPathHolder"))
  (Variables|Default|SetPathHolder _returnvalue))

(fn Setup
  (|CallParentFunction)
  (bind _asgmc_player_controller (Utilities|Casting|CastToGMC_PlayerController (Class|GameplayStatics|GetPlayerControllerfromID)))
  (bind _returnvalue (UserInterface|CreateWidget "/GMCE_Motion/UI/WBP_MotionMatch.WBP_MotionMatch_C" _asgmc_player_controller))
  (UserInterface|Viewport|AddtoViewport _returnvalue 0))

(fn HandleJump
  (params (InputAction :type Input%20Action%20Object%20Reference))
  (if (and (GameplayTags|HasTag (Variables|/Script/GMCExtended.GMCE_OrganicMovementCmp|GetAvailableSolvers (Variables|Default|GetTemplate%20Movement%20Component)) "(TagName=\"Solver.Traversal\")") (not (Class|GMCAbilitySystemComponent|HasAnyTag (Variables|Default|GetAbilitySystemComponent) "(GameplayTags=((TagName=\"State.Dead\"),(TagName=\"State.Respawning\"),(TagName=\"Solver.Traversal\")))")))
    (Class|GMCAbilitySystemComponent|QueueAbility (Variables|Default|GetAbilitySystemComponent) "(TagName=\"Ability.Traverse\")" InputAction)
    (else
      (|CallParentFunction InputAction))))

(fn GetInteractionTransform
  (return (Variables|Default|GetInteractionTransform)))

(fn SetInteractionTransform
  (params (InteractionTransform :type Transform))
  (Variables|Default|SetInteractionTransform InteractionTransform))